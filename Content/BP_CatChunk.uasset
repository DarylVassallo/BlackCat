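; BP_CatChunk is a short-lived physics debris actor, apparently a piece of a cat, that flings itself outward when spawned.
; On BeginPlay it gives its static mesh a random uniform scale and a random linear velocity on each axis.
; After a brief delay it destroys itself, so the chunks clean up automatically.
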(event EventBeginPlay
  (Transformation|SetWorldScale3D (Variables|Default|GetStaticMesh) (Math|Conversions|ToVector(Float) (Math|Random|RandomFloatinRange 0.1 1.0)))
  (Physics|SetPhysicsLinearVelocity (Variables|Default|GetStaticMesh) (Math|Vector|MakeVector (Math|Random|RandomFloatinRange -1.5e+03 1.5e+03) (Math|Random|RandomFloatinRange -1.5e+03 1.5e+03) (Math|Random|RandomFloatinRange -1.5e+03 1.5e+03)) false "None")
  (Utilities|FlowControl|Delay 2.0)
  (Actor|DestroyActor))

(event Collision|EventActorBeginOverlap
  (params (OtherActor :type Actor%20Object%20Reference)))

(event EventTick
  (params (DeltaSeconds :type Float%20%28single-precision%29)))

(fn ConstructionScript)